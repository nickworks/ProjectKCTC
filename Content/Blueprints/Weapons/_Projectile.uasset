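; Base weapon projectile Blueprint that damages what it touches or explodes on contact.
; Sphere overlaps ignore the projectile's owner and actors sharing that owner, then either trigger Explosion or apply point damage to the other actor and destroy the projectile.
; Blocking hits explode or simply destroy it.
; Explosion applies radial damage at its location using the configured radius and damage type, then destroys the projectile.
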(event `self.Sphere.OnComponentBeginOverlap`
  (params (OverlappedComponent :type "PrimitiveComponent Object Reference") (OtherActor :type "Actor Object Reference") (OtherComp :type "PrimitiveComponent Object Reference") (OtherBodyIndex :type Integer) (bFromSweep :type Boolean) (SweepResult :type "HitResult Structure (by ref)"))
  (bind _returnvalue (`self.GetOwner`))
  (if (or (== OtherActor _returnvalue) (== _returnvalue (`self.GetOwner` OtherActor)))
    _
    (elif (`self.explodes`)
      (`self.Explosion`)
      (else
        (`GameplayStatics.ApplyDamage` OtherActor (`KismetMathLibrary.Conv_IntToDouble` (`self.damage amount`)))
        (`self.K2_DestroyActor`)))))

(event `self.Sphere.OnComponentHit`
  (params (HitComponent :type "PrimitiveComponent Object Reference") (OtherActor :type "Actor Object Reference") (OtherComp :type "PrimitiveComponent Object Reference") (NormalImpulse :type "Vector Structure") (Hit :type "HitResult Structure (by ref)"))
  (if (`self.explodes`)
    (`self.Explosion`)
    (else
      (`self.K2_DestroyActor`))))

(event `Explosion`
  (if (`self.explodes`)
    (`GameplayStatics.ApplyRadialDamage` :`BaseDamage` (`KismetMathLibrary.Conv_IntToDouble` (`self.damage amount`)) :`Origin` (`self.K2_GetActorLocation`) :`DamageRadius` (`self.explosion radius`) :`DamageTypeClass` "/Script/Engine.DamageType" :`DamageCauser` null :`InstigatedByController` null)
    (`self.K2_DestroyActor`)
    (else
      (`self.K2_DestroyActor`))))

(fn `UserConstructionScript`)