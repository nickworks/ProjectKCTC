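; Base weapon Blueprint whose Attack stores the player, branches on a Behavior setting to projectile, hitscan or melee, and plays a sound.
; Projectile spawns the configured class aimed at a point along the player's follow-camera forward, passing on its damage amount.
; Hitscan line-traces from that camera and applies point damage.
; Melee opens a brief timed state during which mesh overlaps damage actors, excluding the owner and its possessions.
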(event `Begin Melee`
  (set `self.State` "NewEnumerator3")
  (`KismetSystemLibrary.Delay` 0.2)
  (set `self.State` "NewEnumerator0"))

(event `self.StaticMesh.OnComponentBeginOverlap`
  (params (OverlappedComponent :type "PrimitiveComponent Object Reference") (OtherActor :type "Actor Object Reference") (OtherComp :type "PrimitiveComponent Object Reference") (OtherBodyIndex :type Integer) (bFromSweep :type Boolean) (SweepResult :type "HitResult Structure (by ref)"))
  (bind _returnvalue (`self.GetOwner`))
  (if (`|EnumEquality` (`self.Behavior`) "NewEnumerator2")
    (if (`|EnumEquality` (`self.State`) "NewEnumerator3")
      (if (not (or (== (`self.GetOwner` OtherActor) _returnvalue) (== OtherActor _returnvalue)))
        (`GameplayStatics.ApplyDamage` OtherActor (`KismetMathLibrary.Conv_IntToDouble` (`self.damage amount`)))))))

(fn `Attack`
  (params (`player ref` :type "/Game/Blueprints/HeroPlayer Object Reference"))
  (set `self.Player Ref` `player ref`)
  (switch `/Game/Blueprints/Weapons/WeaponBehavior` (`self.Behavior`)
    (:`NewEnumerator0`
      (`self.AttackProjectile`))
    (:`NewEnumerator1`
      (`self.AttackHitScan`))
    (:`NewEnumerator2`
      (`self.AttackMelee`)))
  (`GameplayStatics.PlaySoundAtLocation` "/Engine/VREditor/Sounds/UI/Selection_Changes.Selection_Changes" (`self.K2_GetActorLocation`) (struct) 1.0 1.0 0.0 null null null))

(fn `AttackHitScan`
  (bind _followcamera (`/Game/Blueprints/HeroPlayer.FollowCamera` (`self.Player Ref`)))
  (bind _returnvalue (`SceneComponent.K2_GetComponentLocation` _followcamera))
  (bind (_outhit _returnvalue_2) (`KismetSystemLibrary.LineTraceSingle` _returnvalue (+ _returnvalue (* (`SceneComponent.GetForwardVector` _followcamera) 2000.0)) "TraceTypeQuery1" false (`|MakeArray` (`self.Player Ref`) :!type "Actor Object Reference")))
  (if _returnvalue_2
    (bind (_bblockinghit _binitialoverlap _time _distance _location _impactpoint _normal _impactnormal _physmat _hitactor _hitcomponent _hitbonename _hititem _faceindex _tracestart _traceend) (`GameplayStatics.BreakHitResult` _outhit))
    (`GameplayStatics.ApplyPointDamage` _hitactor (`KismetMathLibrary.Conv_IntToDouble` (`self.damage amount`)) (`KismetMathLibrary.Normal` (- _traceend _tracestart)) _outhit)))

(fn `AttackMelee`
  (`self.Begin Melee`))

(fn `AttackProjectile`
  (bind _returnvalue (`self.K2_GetActorLocation`))
  (bind _projectile_type (`self.Projectile Type`))
  (bind _followcamera (`/Game/Blueprints/HeroPlayer.FollowCamera` (`self.Player Ref`)))
  (if (`KismetSystemLibrary.IsValidClass` _projectile_type)
    (bind _returnvalue_2 (`|SpawnActorFromClass` _projectile_type (`KismetMathLibrary.MakeTransform` _returnvalue (`KismetMathLibrary.FindLookAtRotation` _returnvalue (+ (`SceneComponent.K2_GetComponentLocation` _followcamera) (* (`SceneComponent.GetForwardVector` _followcamera) 2000.0)))) "Undefined" "OverrideRootScale" (`self.Player Ref`) null))
    (set `/Game/Blueprints/Objects/Projectile.damage amount` (`self.damage amount`) _returnvalue_2)))

(fn `UserConstructionScript`)