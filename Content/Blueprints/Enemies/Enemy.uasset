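; Enemy actor that chases the hero, attacks at close range, and explodes on death with a chance to drop a diamond or fruit.
; BeginPlay spawns an AI controller, sets health from the current level and targets the player's Shadow.
; A delay-driven SetState loop alternates pursuit and attack, using PlayerCollider overlaps as the range check.
; AnyDamage subtracts truncated damage and handles death.
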(event `self.ReceiveAnyDamage`
  (params (Damage :type "Float (single-precision)") (DamageType :type "DamageType Object Reference") (InstigatedBy :type "Controller Object Reference") (DamageCauser :type "Actor Object Reference"))
  (bind _output_get (set `self.health` (- (`self.health`) (`KismetMathLibrary.FTrunc` Damage))))
  (`KismetSystemLibrary.PrintString` (`KismetStringLibrary.Concat_StrStr` (`KismetStringLibrary.Conv_DoubleToString` Damage) " dmg, health now: " (`KismetStringLibrary.Conv_IntToString` (`self.health`))))
  (if (<= _output_get 0)
    (`self.Explode and Spawn Loot`)
    (`self.K2_DestroyActor`)))

(event `self.ReceiveBeginPlay`
  (`self.SpawnDefaultController`)
  (`self.Set attack target to Player`)
  (`self.Move To Player`))

(event `self.ReceivePointDamage`
  (params (Damage :type "Float (single-precision)") (DamageType :type "DamageType Object Reference") (HitLocation :type "Vector Structure") (HitNormal :type "Vector Structure") (HitComponent :type "PrimitiveComponent Object Reference") (BoneName :type Name) (ShotFromDirection :type "Vector Structure") (InstigatedBy :type "Controller Object Reference") (DamageCauser :type "Actor Object Reference") (HitInfo :type "HitResult Structure (by ref)")))

(event `Set State`
  (params (`State of Mind` :type "/Game/Blueprints/Enemies/EnemyStateOfMind Enum" :default "NewEnumerator0"))
  (bind _current_target (`self.current target`))
  (bind _output_get (set `self.State of Mind` `State of Mind`))
  (switch `/Game/Blueprints/Enemies/EnemyStateOfMind` _output_get
    (:`NewEnumerator0`
      (bind _asaicontroller (cast `AIController` (`self.GetController`) :!label _label)
        (:`then`
          (`/Engine/EditorBlueprintResources/StandardMacros.IsValid` _current_target
            (:`Is Valid`
              (`AIBlueprintHelperLibrary.SimpleMoveToActor` _asaicontroller _current_target))
            (:`Is Not Valid`
              _)))
        (:`CastFailed`
          _))
      (`KismetSystemLibrary.Delay` 0.5)
      (if (`self.is close enough to attack`)
        (`self.Set State` "NewEnumerator2")
        (else
          (`self.Set State` "NewEnumerator0"))))
    (:`NewEnumerator2`
      (bind _ashero_player (cast `/Game/Blueprints/HeroPlayer` (`GameplayStatics.GetPlayerCharacter` 0)))
      (`GameplayStatics.ApplyDamage` _ashero_player 1.0)
      (`KismetSystemLibrary.Delay` 0.2)
      (`self.Set State` "NewEnumerator0"))))

(event `Move To Player`
  (goto _label))

(event `self.Player Collider.OnComponentBeginOverlap`
  (params (OverlappedComponent :type "PrimitiveComponent Object Reference") (OtherActor :type "Actor Object Reference") (OtherComp :type "PrimitiveComponent Object Reference") (OtherBodyIndex :type Integer) (bFromSweep :type Boolean) (SweepResult :type "HitResult Structure (by ref)"))
  (cast `/Game/Blueprints/HeroPlayer` OtherActor)
  (set `self.is close enough to attack` true))

(event `self.Player Collider.OnComponentEndOverlap`
  (params (OverlappedComponent :type "PrimitiveComponent Object Reference") (OtherActor :type "Actor Object Reference") (OtherComp :type "PrimitiveComponent Object Reference") (OtherBodyIndex :type Integer))
  (cast `/Game/Blueprints/HeroPlayer` OtherActor)
  (set `self.is close enough to attack` false))

(fn `Explode and Spawn Loot`
  (bind _returnvalue (`self.K2_GetActorLocation`))
  (`NiagaraFunctionLibrary.SpawnSystemAtLocation` (`self.explosion FX`) (`self.K2_GetActorLocation`))
  (if (< (`KismetMathLibrary.RandomFloatInRange` 0.0 1.0) (`self.chance of diamonds`))
    (`|SpawnActorFromClass` "/Game/Blueprints/Objects/Diamond.Diamond_C" (`KismetMathLibrary.MakeTransform` _returnvalue) "Undefined" "OverrideRootScale" null null)
    (elif (< (`KismetMathLibrary.RandomFloatInRange` 0.0 1.0) (`self.chance of fruit`))
      (`|SpawnActorFromClass` "/Game/Blueprints/Objects/BigFruit.BigFruit_C" (`KismetMathLibrary.MakeTransform` _returnvalue) "Undefined" "OverrideRootScale" null null))))

(fn `Set attack target to Player`
  (bind _ashero_player (cast `/Game/Blueprints/HeroPlayer` (`GameplayStatics.GetPlayerPawn` 0)))
  (set `self.health` (+ (`/Game/Blueprints/TheGameInstance.current level` (`/Game/Blueprints/HeroPlayer.the Game Instance` _ashero_player)) 3))
  (set `self.current target` (`/Game/Blueprints/HeroPlayer.shadow` _ashero_player)))

(fn `UserConstructionScript`)