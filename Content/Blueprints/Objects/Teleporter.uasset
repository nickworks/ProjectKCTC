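; Teleporter object that sends the player to either the next combat level or the main camp, based on its destination setting.
; Overlapping its trigger volume enables input and has the game instance note the hero's current weapons; leaving disables input.
; Pressing Interact calls the matching teleport function on the game instance.
; The construction script labels it with the destination name; a bounce timeline for the animated component exists but never runs.
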(event `self.ReceiveBeginPlay`)

(event `self.Trigger Volume.OnComponentBeginOverlap`
  (params (OverlappedComponent :type "PrimitiveComponent Object Reference") (OtherActor :type "Actor Object Reference") (OtherComp :type "PrimitiveComponent Object Reference") (OtherBodyIndex :type Integer) (bFromSweep :type Boolean) (SweepResult :type "HitResult Structure (by ref)"))
  (bind _ashero_player (cast `/Game/Blueprints/HeroPlayer` OtherActor))
  (`self.EnableInput` (`GameplayStatics.GetPlayerController` 0))
  (`/Game/Blueprints/TheGameInstance.Take Note of Current Weapons` (`/Game/Blueprints/HeroPlayer.the Game Instance` _ashero_player)))

(event `self.Trigger Volume.OnComponentEndOverlap`
  (params (OverlappedComponent :type "PrimitiveComponent Object Reference") (OtherActor :type "Actor Object Reference") (OtherComp :type "PrimitiveComponent Object Reference") (OtherBodyIndex :type Integer))
  (cast `/Game/Blueprints/HeroPlayer` OtherActor)
  (`self.DisableInput` (`GameplayStatics.GetPlayerController` 0)))

(event `InputAction|Interact` :consume false
  (params (Key :type "Key Structure"))
  (:`Pressed`
    (bind _asthe_game_instance (cast `/Game/Blueprints/TheGameInstance` (`GameplayStatics.GetGameInstance`)))
    (switch `/Game/Blueprints/Objects/TeleporterType` (`self.Teleporter Destination`)
      (:`NewEnumerator0`
        (`/Game/Blueprints/TheGameInstance.Teleport to Next Level` _asthe_game_instance))
      (:`NewEnumerator1`
        (`/Game/Blueprints/TheGameInstance.Teleport to Main Camp` _asthe_game_instance)))))

(fn `UserConstructionScript`
  (`TextRenderComponent.K2_SetText` (`self.TextRender`) (`KismetTextLibrary.Conv_StringToText` (`KismetStringLibrary.Concat_StrStr` "Teleport to \n" (`|GetEnumeratorNameAsString` (`self.Teleporter Destination`))))))