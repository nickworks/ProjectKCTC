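; WeaponExchange is a world pickup that holds one weapon and lets the player swap for it.
; On BeginPlay it spawns WeaponType, attaches it to itself and hides its prompt text.
; A HeroPlayer entering the sphere enables input and shows the prompt, and leaving reverses both.
; Interact passes the held weapon to the player's WeaponPickupSwap, then displays the returned weapon and updates the prompt with its category and name.
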(event `self.Sphere.OnComponentBeginOverlap`
  (params (OverlappedComponent :type "PrimitiveComponent Object Reference") (OtherActor :type "Actor Object Reference") (OtherComp :type "PrimitiveComponent Object Reference") (OtherBodyIndex :type Integer) (bFromSweep :type Boolean) (SweepResult :type "HitResult Structure (by ref)"))
  (cast `/Game/Blueprints/HeroPlayer` OtherActor)
  (`self.EnableInput` (`GameplayStatics.GetPlayerController` 0))
  (`SceneComponent.SetVisibility` (`self.TextRender`) true false))

(event `self.Sphere.OnComponentEndOverlap`
  (params (OverlappedComponent :type "PrimitiveComponent Object Reference") (OtherActor :type "Actor Object Reference") (OtherComp :type "PrimitiveComponent Object Reference") (OtherBodyIndex :type Integer))
  (cast `/Game/Blueprints/HeroPlayer` OtherActor)
  (`self.DisableInput` (`GameplayStatics.GetPlayerController` 0))
  (`SceneComponent.SetVisibility` (`self.TextRender`) false false :!label _label))

(event `self.ReceiveBeginPlay`
  (bind _returnvalue (`|SpawnActorFromClass` (`self.weapon type`) (`KismetMathLibrary.MakeTransform` (0.0 0.0 0.0)) "Undefined" "OverrideRootScale" null null))
  (`self.Equip Weapon` _returnvalue)
  (goto _label))

(event `InputAction|Interact`
  (params (Key :type "Key Structure"))
  (:`Pressed`
    (bind _ashero_player (cast `/Game/Blueprints/HeroPlayer` (`GameplayStatics.GetPlayerCharacter` 0)))
    (bind _the_old_weapon (`/Game/Blueprints/HeroPlayer.Weapon Pickup Swap` _ashero_player (`self.held weapon`)))
    (`self.Equip Weapon` _the_old_weapon)))

(fn `Equip Weapon`
  (params (`held weapon` :type "/Game/Blueprints/Weapons/_Weapon Object Reference"))
  (bind _output_get (set `self.held weapon` `held weapon`))
  (`self.SetActorHiddenInGame` _output_get false)
  (`TextRenderComponent.K2_SetText` (`self.TextRender`) (`KismetTextLibrary.Conv_StringToText` (`KismetStringLibrary.Concat_StrStr` "swap " (`|GetEnumeratorNameAsString` (`/Game/Blueprints/Weapons/_Weapon.Default Category` _output_get)) " \nfor " (`/Game/Blueprints/Weapons/_Weapon.Weapon Name` _output_get))))
  (`self.K2_AttachToActor` _output_get self "None" "SnapToTarget" "SnapToTarget" "SnapToTarget" false))

(fn `UserConstructionScript`
  (`TextRenderComponent.K2_SetText` (`self.TextRender`) (`KismetTextLibrary.Conv_StringToText` (`KismetSystemLibrary.GetClassDisplayName` (`self.weapon type`)))))