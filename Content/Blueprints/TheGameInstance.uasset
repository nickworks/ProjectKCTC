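; Game instance that holds persistent run state (player health, healing fruit, diamonds, level counter) and handles level travel.
; LoadLevel shows a loader widget, waits a second, then unloads the current streamed level and loads the next by name.
; Next-level teleports repeat the Combat level until the counter reaches six, then load FinalBoss; another teleport loads Camp.
; Fruit items fully or partially heal, and ResetGame restores starting values.
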(event `Load Level`
  (params (`next level` :type Name))
  (bind _returnvalue (`|CreateWidget` "/Game/Blueprints/GUI/LoaderGUI.LoaderGUI_C"))
  (`UserWidget.AddToPlayerScreen` _returnvalue 1000)
  (`KismetSystemLibrary.Delay` 1.0)
  (`GameplayStatics.UnloadStreamLevel` (`self.current level name`))
  (bind _output_get (set `self.current level name` `next level`))
  (`GameplayStatics.LoadStreamLevel` _output_get true))

(fn `Heal Big`
  (bind _fruit_big (`self.fruit big`))
  (if (> _fruit_big 0)
    (set `self.fruit big` (- _fruit_big 1))
    (set `self.player health` (`self.max player health`))
    (`KismetSystemLibrary.PrintString` "Recovery Item used!")))

(fn `Heal Small`
  (bind _fruit_small (`self.fruit small`))
  (if (> _fruit_small 0)
    (set `self.fruit small` (- _fruit_small 1))
    (set `self.player health` (`KismetMathLibrary.Min` (`self.max player health`) (+ (`self.player health`) 4)))
    (`KismetSystemLibrary.PrintString` "Recovery Item used!")))

(fn `Reset Game`
  (set `self.current level` 0)
  (bind _output_get (set `self.max player health` 12))
  (set `self.player health` _output_get)
  (set `self.fruit small` 0)
  (set `self.fruit big` 0)
  (set `self.diamonds` 0))

(fn `Teleport to Main Camp`
  (`self.Load Level` "Camp"))

(fn `Teleport to Next Level`
  (bind _output_get (set `self.current level` (+ (`self.current level`) 1)))
  (if (>= _output_get 6)
    (`KismetSystemLibrary.PrintString` "Go to final boss?")
    (`self.Load Level` "FinalBoss")
    (else
      (`KismetSystemLibrary.PrintString` (`KismetStringLibrary.Concat_StrStr` "going to level #" (`KismetStringLibrary.Conv_IntToString` (`self.current level`))))
      (`self.Load Level` "Combat"))))